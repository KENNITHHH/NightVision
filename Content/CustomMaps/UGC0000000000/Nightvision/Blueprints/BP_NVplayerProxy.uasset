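; Pavlov player proxy that gives each pawn toggleable night vision goggles.
; On spawn it attaches the interaction root to the camera and the goggle model to the head bone, showing one of two models by team.
; A trigger press by the owner replicates to the server and flips IsNVOn.
; Its OnRep rotates the goggles, plays sound, sets emissive glow, toggles the effect sphere and recolors inventory laser beams green or red.
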(event `self.ReceiveBeginPlay`
  (bind _nv_goggles (`self.NV_Goggles`))
  (bind _nv_gogglesmono (`self.NV_GogglesMono`))
  ;[0 1 0] On Player Spawning - Attach Nightvision Components to Pawn Skeleton and Camera
  ;;[1 1 1] When Spawning reset all Laser Colors to Red
  (`self.ToggleLaserColor` false)
  ;;[1 1 1] CLIENT - Nightvision Interaction Box - Snapping to Camera
  (`KismetSystemLibrary.Delay` 1.0)
  (`SceneComponent.K2_AttachToComponent` (`self.NV_BaseRoot`) (`self.GetComponentByClass` (`self.GetPawn`) "/Script/Engine.CameraComponent") "head" "SnapToTarget" "SnapToTarget" "KeepRelative" true)
  ;;[1 1 1] Nightvision Model - Snapping to Head Bone - Setting Location and Rotation offset
  (`SceneComponent.K2_AttachToComponent` (`self.NV_ModelRoot`) (`self.GetPlayerSkeleton`) "head" "SnapToTarget" "SnapToTarget" "KeepRelative" true)
  (`SceneComponent.K2_AddRelativeLocation` (`self.NV_ModelRoot`) (13.0 12.0 0.0) false false)
  (`SceneComponent.K2_AddRelativeRotation` (`self.NV_ModelRoot`) (struct :`Yaw` -135.0) false false)
  ;;[1 1 1] Nightvision Hide per Team - TeamID 0 = Green - TeamID 1 = Amber/Red
  (bind _playerstatus (`PavlovProxyStatics.GetPavlovPlayerStatusByPawn` (`self.GetPawn`)))
  (if (== (`.TeamId` (break `PavlovPlayerStatus` _playerstatus)) 0)
    (`SceneComponent.SetVisibility` _nv_goggles true false)
    (`SceneComponent.SetVisibility` _nv_gogglesmono false false)
    (else
      (`SceneComponent.SetVisibility` _nv_goggles false false)
      (`SceneComponent.SetVisibility` _nv_gogglesmono true false))))

(event `self.NV_ToggleBox.OnInteractBoxClient`
  (params (InteractType :type "EInteractType Enum" :default "Grabbed") (HandProxy :type "Pavlov_HandProxy Object Reference") (InteractBox :type "Pavlov_InteractBox Object Reference"))
  ;[0 1 0] On Player Spawning - Attach Nightvision Components to Pawn Skeleton and Camera
  ;;[1 1 1] Nightvision Toggling Interaction
  (if (and (`|EnumEquality` InteractType "Trigger") (== (`self.GetPawn` (`Pavlov_HandProxy.GetPlayerProxy` HandProxy)) (`self.GetPawn`)))
    (`Pavlov_HandProxy.ReplicateInteract_Server` HandProxy InteractType InteractBox)))

(event `self.NV_ToggleBox.OnInteractBoxServer`
  (params (InteractType :type "EInteractType Enum" :default "Grabbed") (HandProxy :type "Pavlov_HandProxy Object Reference") (InteractBox :type "Pavlov_InteractBox Object Reference"))
  ;[0 1 0] On Player Spawning - Attach Nightvision Components to Pawn Skeleton and Camera
  ;;[1 1 1] Nightvision Toggling Interaction
  (`self.ToggleNightvision`))

(event `CLIENT_EnableSphere`
  ;[0 1 0] On Player Spawning - Attach Nightvision Components to Pawn Skeleton and Camera
  ;;[1 1 1] Toggling Clientside Effect Sphere
  (`SceneComponent.SetHiddenInGame` (`self.NV_EffectSphere`) false false))

(event `ToggleNightvision`
  ;[0 1 0] On Player Spawning - Attach Nightvision Components to Pawn Skeleton and Camera
  (set `self.IsNV_On?` (not (`self.IsNV_On?`))))

(event `CLIENT_DisableSphere`
  ;[0 1 0] On Player Spawning - Attach Nightvision Components to Pawn Skeleton and Camera
  ;;[1 1 1] Toggling Clientside Effect Sphere
  (`SceneComponent.SetHiddenInGame` (`self.NV_EffectSphere`) true false))

(event `ToggleLaserColor`
  (params (SetGreen :type Boolean))
  ;[0 1 0] On Player Spawning - Attach Nightvision Components to Pawn Skeleton and Camera
  ;;[1 1 1] Set Laser Colors - Green - Red
  (bind _items (`self.GetAllItems`))
  (for _array_element _items
    (for _array_element_2 (`self.GetAttachedActors` (`.Item` (break `PlayerItem` _array_element)))
      (if (`KismetStringLibrary.Contains` (`KismetSystemLibrary.GetDisplayName` _array_element_2) "laser")
        (for _array_element_3 (`self.K2_GetComponentsByClass` _array_element_2 "/Script/Engine.StaticMeshComponent")
          (if (`KismetStringLibrary.Contains` (`KismetSystemLibrary.GetDisplayName` _array_element_3) "SM_Laser_")
            _
            (elif (and (`KismetSystemLibrary.IsValid` _array_element_3) SetGreen)
              (`PrimitiveComponent.SetMaterial` _array_element_3 0 "/Game/CustomMaps/UGC0000000000/Nightvision/Materials/MI_LaserBeamGreen.MI_LaserBeamGreen")
              (else
                (`PrimitiveComponent.SetMaterial` _array_element_3 0 "/Game/CustomMaps/UGC0000000000/Nightvision/Materials/MI_LaserBeamRed.MI_LaserBeamRed")))))))))

(fn `OnRep_NV_On?`
  (bind _nv_modelroot (`self.NV_ModelRoot`))
  (bind _nvgogglesmaterial (`self.NVGogglesMaterial`))
  (bind _returnvalue (`SceneComponent.K2_GetComponentLocation` (`self.NV_ModelRoot`)))
  ;[0 1 0 10] Rotating NV Goggles Model - Playing NV Sounds - Toggling NV Goggles Lights and Color
  (if (`self.IsNV_On?`)
    (`SceneComponent.K2_AddRelativeRotation` _nv_modelroot (struct :`Yaw` 135.0) false false)
    (`GameplayStatics.PlaySoundAtLocation` "/Game/CustomMaps/UGC0000000000/Nightvision/Sounds/C_TurnNVOn.C_TurnNVOn" _returnvalue (struct) 1.0 1.0 0.0 null null null)
    (`MaterialInstanceDynamic.SetScalarParameterValue` _nvgogglesmaterial "EmissivePower" 5.0)
    (`MaterialInstanceDynamic.SetScalarParameterValue` (`self.NVGogglesMonoMaterial`) "EmissivePower" 5.0)
    (`self.CLIENT_EnableSphere`)
    (`self.ToggleLaserColor` true)
    (else
      (`SceneComponent.K2_AddRelativeRotation` _nv_modelroot (struct :`Yaw` -135.0) false false)
      (`GameplayStatics.PlaySoundAtLocation` "/Game/CustomMaps/UGC0000000000/Nightvision/Sounds/C_TurnNVOff.C_TurnNVOff" _returnvalue (struct) 1.0 1.0 0.0 null null null)
      (`MaterialInstanceDynamic.SetScalarParameterValue` _nvgogglesmaterial "EmissivePower" 0.0)
      (`MaterialInstanceDynamic.SetScalarParameterValue` (`self.NVGogglesMonoMaterial`) "EmissivePower" 0.0)
      (`self.CLIENT_DisableSphere`)
      (`self.ToggleLaserColor` false))))

(fn `UserConstructionScript`
  ;[0 1 0 10] Creating Dynamic Material Instance to Increase/Decreate the NV Model's Light
  (bind _returnvalue (`PrimitiveComponent.CreateDynamicMaterialInstance` (`self.NV_Goggles`) 0 "/Game/CustomMaps/UGC0000000000/Nightvision/Materials/MI_NVgoggles.MI_NVgoggles" "None"))
  (set `self.NVGogglesMaterial` _returnvalue)
  (bind _returnvalue_2 (`PrimitiveComponent.CreateDynamicMaterialInstance` (`self.NV_GogglesMono`) 0 "/Game/CustomMaps/UGC0000000000/Nightvision/Materials/MI_NVgogglesMono.MI_NVgogglesMono" "None"))
  (set `self.NVGogglesMonoMaterial` _returnvalue_2))